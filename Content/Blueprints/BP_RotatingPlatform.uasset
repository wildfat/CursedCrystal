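; Rotating platform with four crystal batteries, whose beam color follows the currently selected crystal and is broadcast through OnColorChanged.
; A looping 30-second timer randomizes the crystal effects and refreshes the beam.
; A BP_CrystalCharacter overlapping the box triggers a timeline quarter turn that advances the selection and hides the beam until finished.
; The overlap also deals radial damage ignoring that character and applies a radial impulse to its overlapping component.
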(event OnComponentBeginOverlap(Box)
  (params (OverlappedComponent :type Primitive%20Component%20Object%20Reference) (OtherActor :type Actor%20Object%20Reference) (OtherComp :type Primitive%20Component%20Object%20Reference) (OtherBodyIndex :type Integer) (bFromSweep :type Boolean) (SweepResult :type Hit%20Result%20Structure%20%28by%20ref%29))
  (bind _location (Collision|BreakHitResult SweepResult))
  (bind _asbp_crystal_character (Utilities|Casting|CastToBP_CrystalCharacter OtherActor))
  (CallFunction|RotatePlatform)
  (Game|Damage|ApplyRadialDamage 1e+01 _location 1e+03 0 (Utilities|Array|MakeArray _asbp_crystal_character) _asbp_crystal_character (Game|GetPlayerController 0) true "ECC_Visibility")
  (Physics|AddRadialImpulse OtherComp _location 1e+03 1e+04 "RIF_Linear" true))

(event Custom|RotatePlatform
  (bind _p_beam (Variables|Default|GetP_Beam))
  (if (not (Variables|Default|GetIsPlatformMoving))
    (Variables|Default|SetRelative%20Rotation%20Z%20%28Yaw%29 (.yaw (Variables|/Script/Engine.SceneComponent|GetRelativeRotation (Variables|Default|GetPlatformMesh))))
    (Variables|Default|SetIsPlatformMoving true)
    (Rendering|SetVisibility _p_beam false false)
    (Components|Activation|Deactivate _p_beam)
    (Utilities|FlowControl|Sequence
      (:then_0
        (bind _rotate (Timeline|Timeline_0 SetNewTime)
          (:Update
            (Transformation|SetRelativeRotation (Variables|Default|GetPlatformMesh) (Math|Rotator|MakeRotator 0.0 0.0 (+ (* _rotate 9e+01) (Variables|Default|GetRelative%20Rotation%20Z%20%28Yaw%29))) false false))
          (:Finished
            (Variables|Default|SetIsPlatformMoving false)
            (Math|Integer|IncrementInt (Variables|Default|GetCurrentPosition)
              (:%20%20
                (if (> (Variables|Default|GetCurrentPosition) 3)
                  (Variables|Default|SetCurrentPosition 0))
                (CallFunction|SetPlatformEffect))))))
      (:then_1
        (Timeline|Timeline_0 Play)))))

(event Custom|SwapCrystals
  (Utilities|Time|SetTimerbyEvent (delegate Custom|SwapCrystals) 3e+01 true)
  (for _array_element (Variables|Default|GetAs%20BP%20Crystal%20Battery)
    (Default|SetCrystalEffect _array_element (Utilities|Enum|ByteToEnumE_Effects (Math|Conversions|ToByte(Integer) (Math|Random|RandomIntegerinRange 1 4)))))
  (CallFunction|SetPlatformEffect))

(event Custom|SetPlatformEffect
  (bind _p_beam (Variables|Default|GetP_Beam))
  (Variables|Default|SetCurrentColor (Variables|/Game/Blueprints/BP_CrystalBattery.BP_CrystalBattery_C|GetCurrentEffect (Utilities|Array|Get(acopy) (Variables|Default|GetAs%20BP%20Crystal%20Battery) (Variables|Default|GetCurrentPosition))))
  (Rendering|SetVisibility _p_beam true false)
  (Components|Activation|Activate _p_beam true)
  (Effects|Components|ParticleSystem|SetVectorParameter _p_beam "Color" (Math|Conversions|ToVector(LinearColor) (Utilities|Select :Index (Variables|Default|GetCurrentColor) :NewEnumerator5 "" :NewEnumerator0 "(R=1.000000,G=0.000000,B=0.000000,A=1.000000)" :NewEnumerator1 "(R=0.000000,G=1.000000,B=0.000000,A=1.000000)" :NewEnumerator2 "(R=0.000000,G=0.000000,B=1.000000,A=1.000000)" :NewEnumerator3 "(R=1.000000,G=1.000000,B=0.000000,A=1.000000)")))
  (Default|CallOnColorChanged (Variables|Default|GetCurrentColor)))

(event EventBeginPlay
  ;[1 1 1] Begin play
  (Effects|Components|ParticleSystem|SetVectorParameter (Variables|Default|GetP_Beam) "Color" (Math|Conversions|ToVector(LinearColor) (Utilities|Array|Get(acopy) (Variables|Default|GetValue))))
  (for _array_element (Utilities|Array|MakeArray (Variables|Default|GetChildActor) (Variables|Default|GetChildActor1) (Variables|Default|GetChildActor2) (Variables|Default|GetChildActor3))
    (bind _asbp_crystal_battery (Utilities|Casting|CastToBP_CrystalBattery (Variables|/Script/Engine.ChildActorComponent|GetChildActor _array_element)))
    (Utilities|Array|Add (Variables|Default|GetAs%20BP%20Crystal%20Battery) _asbp_crystal_battery))
  (CallFunction|SwapCrystals))

(fn ConstructionScript)