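; Main crystal actor that shakes with growing intensity while unstable and stabilizes when all its linked platforms share one color.
; Platform color-change events trigger a match check, which tints the glass dynamic material to that color or black and, on a match, resets shake and countdown.
; A looping timer either applies the crystal's color effect to the character or jitters the mesh rotation while counting down to an explosion, whose branch is empty.
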(event Custom|ShakeMeshTimer
  ;[1 1 1] Shake
  (Utilities|Time|SetTimerbyEvent (delegate Custom|ShakeMeshTimer) 0.02 true)
  (if (Variables|Default|GetIsStabylazed)
    (Default|SetCrystalEffect (Variables|Default|GetR_Character) (Variables|Default|GetCurrentColor))
    (else
      (Transformation|SetRelativeRotation (Variables|Default|GetMainSection) (Math|Rotator|MakeRotator (Math|Random|RandomFloatinRange (Variables|Default|GetMinShake) (Variables|Default|GetMaxShake)) (Math|Random|RandomFloatinRange (Variables|Default|GetMinShake) (Variables|Default|GetMaxShake)) (Math|Random|RandomFloatinRange (Variables|Default|GetMinShake) (Variables|Default|GetMaxShake))) false false)
      (Variables|Default|SetExposionTimer (- (Variables|Default|GetExposionTimer) 0.01))
      (Variables|Default|SetMinShake (- (Variables|Default|GetMinShake) 0.01))
      (Variables|Default|SetMaxShake (+ (Variables|Default|GetMaxShake) 0.01))
      (if (<= (Variables|Default|GetExposionTimer) 0.0) ; Exposion
        _))))

(event Custom|ColorChanged
  (params (NewParam :type E_Effects%20Enum :default "NewEnumerator5"))
  (bind _output_get (Variables|Default|SetIsStabylazed (CallFunction|CheckAllPlatformsColor)))
  (if _output_get
    (CallFunction|SetCrystalStabilized NewParam)
    (else
      (Rendering|Material|SetVectorParameterValue :self (Variables|Default|GetMaterialInstance) :ParameterName "ColorGlass" :!class /Script/Engine.MaterialInstanceDynamic))))

(event Custom|SetCrystalStabilized
  (params (NewParam :type E_Effects%20Enum :default "NewEnumerator5"))
  ;[1 1 1] Set Stabilised
  (bind _output_get (Variables|Default|SetCurrentColor NewParam))
  (Rendering|Material|SetVectorParameterValue (Variables|Default|GetMaterialInstance) "ColorGlass" (Utilities|Select :Index _output_get :NewEnumerator5 "" :NewEnumerator0 "(R=1.000000,G=0.000000,B=0.000000,A=1.000000)" :NewEnumerator1 "(R=0.000000,G=1.000000,B=0.000000,A=1.000000)" :NewEnumerator2 "(R=0.000000,G=0.000000,B=1.000000,A=1.000000)" :NewEnumerator3 "(R=1.000000,G=1.000000,B=0.000000,A=1.000000)") :!class /Script/Engine.MaterialInstanceDynamic)
  (Variables|Default|SetExposionTimer 5.0)
  (Variables|Default|SetMinShake -1.0)
  (Variables|Default|SetMaxShake 1.0)
  (Transformation|SetRelativeRotation (Variables|Default|GetMainSection) "0, 0, 0" false false))

(event EventBeginPlay
  ;[1 1 1] Begin play
  (bind _returnvalue (Rendering|Material|CreateDynamicMaterialInstance (Variables|Default|GetMainSection) 0 "/Game/StarterContent/Materials/M_Glass_Inst.M_Glass_Inst" "None" :!class /Script/Engine.PrimitiveComponent))
  (Variables|Default|SetMaterialInstance _returnvalue)
  (CallFunction|ShakeMeshTimer)
  (for _array_element (Variables|Default|GetPlatforms_Ref)
    (EventDispatchers|BindEventtoOnColorChanged _array_element (delegate Custom|ColorChanged))))

(fn ConstructionScript)

(fn CheckAllPlatformsColor
  (LocalVariables|SetNewLocalVar_0 (Variables|/Game/Blueprints/BP_RotatingPlatform.BP_RotatingPlatform_C|GetCurrentColor (Utilities|Array|Get(acopy) (Variables|Default|GetPlatforms_Ref))))
  (for _array_element (Variables|Default|GetPlatforms_Ref)
    (if (not (Utilities|Enum|Equal(Enum) (Variables|/Game/Blueprints/BP_RotatingPlatform.BP_RotatingPlatform_C|GetCurrentColor _array_element) (LocalVariables|GetNewLocalVar_0)))
      (return false)))
  (return true))