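; Rotating platform actor that cycles through four positions, changing its beam color and announcing each change through OnColorChanged.
; The construction script tints four objects with dynamic material instances.
; RotatePlatform ignores calls while moving, hides the beam, and turns the mesh by timeline-driven yaw relative to its current angle.
; On finish it advances the wrapping position, maps it to an effect color and restores the beam; hover events toggle a point light.
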(event Custom|RotatePlatform
  (bind _p_beam (Variables|Default|GetP_Beam))
  (bind _p_beam_2 (Variables|Default|GetP_Beam))
  (if (not (Variables|Default|GetIsPlatformMoving))
    (Variables|Default|SetRelative%20Rotation%20Z%20%28Yaw%29 (.yaw (Variables|/Script/Engine.SceneComponent|GetRelativeRotation (Variables|Default|GetPlatformMesh))))
    (Variables|Default|SetIsPlatformMoving true)
    (Rendering|SetVisibility _p_beam_2 false false)
    (Components|Activation|Deactivate _p_beam_2)
    (Utilities|FlowControl|Sequence
      (:then_0
        (bind _rotate (Timeline|Timeline_0 SetNewTime)
          (:Update
            (Transformation|SetRelativeRotation (Variables|Default|GetPlatformMesh) (Math|Rotator|MakeRotator 0.0 0.0 (+ (* _rotate 45.0) (Variables|Default|GetRelative%20Rotation%20Z%20%28Yaw%29))) false false))
          (:Finished
            (Variables|Default|SetIsPlatformMoving false)
            (Math|Integer|IncrementInt (Variables|Default|GetCurrentPosition)
              (:%20%20
                (if (> (Variables|Default|GetCurrentPosition) 3)
                  (Variables|Default|SetCurrentPosition 0))
                (bind _output_get (Variables|Default|SetCurrentColor (Utilities|Enum|ByteToEnumE_Effects (Math|Conversions|ToByte(Integer) (Variables|Default|GetCurrentPosition)))))
                (Rendering|SetVisibility _p_beam true false)
                (Components|Activation|Activate _p_beam true)
                (Effects|Components|ParticleSystem|SetVectorParameter _p_beam "Color" (Math|Conversions|ToVector(LinearColor) (Utilities|Select :Index _output_get :NewEnumerator5 "" :NewEnumerator0 "(R=1.000000,G=0.000000,B=0.000000,A=1.000000)" :NewEnumerator1 "(R=0.000000,G=1.000000,B=0.000000,A=1.000000)" :NewEnumerator2 "(R=0.000000,G=0.000000,B=1.000000,A=1.000000)" :NewEnumerator3 "(R=1.000000,G=1.000000,B=0.000000,A=1.000000)")))
                (Default|CallOnColorChanged))))))
      (:then_1
        (Timeline|Timeline_0 Play)))))

(event Custom|PlatformHovered
  (Rendering|Components|Light|SetIntensity (Variables|Default|GetPointLight) 5e+03))

(event Custom|PlatformUnhobered
  (Rendering|Components|Light|SetIntensity (Variables|Default|GetPointLight) 0.0))

(event EventBeginPlay
  ;[1 1 1] Begin play
  (Effects|Components|ParticleSystem|SetVectorParameter (Variables|Default|GetP_Beam) "Color" (Math|Conversions|ToVector(LinearColor) (Utilities|Array|Get(acopy) (Variables|Default|GetValue))))
  (Default|CallOnColorChanged))

(fn ConstructionScript
  (for (_array_element _array_index) (Utilities|Array|MakeArray (Variables|Default|GetObject0) (Variables|Default|GetObject1) (Variables|Default|GetObject2) (Variables|Default|GetObject3))
    (bind _returnvalue (Rendering|Material|CreateDynamicMaterialInstance _array_element 0 "/Game/Materials/NewMaterial_Inst.NewMaterial_Inst" "None" :!class /Script/Engine.PrimitiveComponent))
    (Rendering|Material|SetVectorParameterValue _returnvalue "Color" (Utilities|Array|Get(acopy) (Variables|Default|GetValue) _array_index) :!class /Script/Engine.MaterialInstanceDynamic)))