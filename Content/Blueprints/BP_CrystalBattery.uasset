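; Crystal battery Blueprint that shows its current crystal effect as the color of its glass mesh.
; BeginPlay creates a dynamic glass material set to black, and SetCrystalEffect stores the effect and recolors it red, green, blue, yellow or black.
; DecreaseEnergy is meant to drain energy through a self-referencing timer, but its delay is zero and the code that refills energy and starts it is disconnected.
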(event Custom|DecreaseEnergy
  (Utilities|Time|SetTimerbyEvent (delegate Custom|DecreaseEnergy) 0.0)
  (if (Variables|Default|GetCondition)
    (Variables|Default|SetCurrentEnergy (- (Variables|Default|GetCurrentEnergy) 0.1))))

(event Custom|SetCrystalEffect
  (params (NewParam :type E_Effects%20Enum :default "NewEnumerator5"))
  (bind _output_get (Variables|Default|SetCurrentEffect NewParam))
  (Rendering|Material|SetVectorParameterValue (Variables|Default|GetDynamicMaterial) "ColorGlass" (Utilities|Select :Index _output_get :NewEnumerator5 "" :NewEnumerator0 "(R=1.000000,G=0.000000,B=0.000000,A=1.000000)" :NewEnumerator1 "(R=0.000000,G=1.000000,B=0.000000,A=1.000000)" :NewEnumerator2 "(R=0.000000,G=0.000000,B=1.000000,A=1.000000)" :NewEnumerator3 "(R=1.000000,G=1.000000,B=0.000000,A=1.000000)") :!class /Script/Engine.MaterialInstanceDynamic))

(event EventBeginPlay
  (bind _returnvalue (Rendering|Material|CreateDynamicMaterialInstance (Variables|Default|GetStaticMesh) 0 "/Game/StarterContent/Materials/M_Glass_Inst.M_Glass_Inst" "None" :!class /Script/Engine.PrimitiveComponent))
  (bind _output_get (Variables|Default|SetDynamicMaterial _returnvalue))
  (Rendering|Material|SetVectorParameterValue :self _output_get :ParameterName "ColorGlass" :!class /Script/Engine.MaterialInstanceDynamic))

(fn ConstructionScript)