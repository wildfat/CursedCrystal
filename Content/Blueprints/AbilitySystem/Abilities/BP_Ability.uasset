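; BP_Ability is an ability Blueprint that tracks a capacity pool, which drains and restores.
; Reduce Ability Capacity subtracts a given amount while capacity is above zero and reports whether the ability can still be used.
; RestoreAbility adds a small fixed step per call while below the maximum and reports whether more restoring remains.
; Neither function clamps the result, and the event graph is empty, so calls must come from elsewhere.
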(event EventBeginPlay)

(event Collision|EventActorBeginOverlap
  (params (OtherActor :type Actor%20Object%20Reference)))

(event EventTick
  (params (DeltaSeconds :type Float%20%28single-precision%29)))

(fn ConstructionScript)

(fn ReduceAbilityCapacity
  (if (> (Variables|Default|GetCurrentCapacity) 0.0)
    (bind _output_get (Variables|Default|SetCurrentCapacity (- (Variables|Default|GetCurrentCapacity) (Variables|Default|GetValueToReduce))))
    (return _output_get (> (Variables|Default|GetCurrentCapacity) 0.0))))

(fn RestoreAbility
  (if (< (Variables|Default|GetCurrentCapacity) (Variables|Default|GetMaxCapacity))
    (bind _output_get (Variables|Default|SetCurrentCapacity (+ (Variables|Default|GetCurrentCapacity) 0.05)))
    (return _output_get (< (Variables|Default|GetCurrentCapacity) (Variables|Default|GetMaxCapacity)))))