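; Ability manager owned by BP_CrystalCharacter that tracks the character's abilities and their capacity.
; On BeginPlay it spawns an actor for each class in the Abilities map, owned by the character, and stores them in AllAbilities.
; The character's OnAbilitySwitched event sets SelectedAbility by matching ability type.
; OnAbilityUsing reduces the selected ability's capacity and reports usability, while OnAbilityRestoring restores an ability looked up by type.
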(event Custom|OnAbilitySwitched_Event_0
  (params (NewParam :type E_Effects%20Enum :default "NewEnumerator5"))
  (for _array_element (Variables|Default|GetAllAbilities)
    (if (Utilities|Enum|Equal(Enum) (.type (Variables|/Game/Blueprints/AbilitySystem/Abilities/BP_Ability.BP_Ability_C|GetAbilityInfo _array_element)) NewParam)
      (Variables|Default|SetSelectedAbility _array_element))))

(event EventBeginPlay
  (bind _astop_down_character (Utilities|Casting|CastToBP_CrystalCharacter (Components|GetOwner)))
  (bind _output_get (Variables|Default|SetR_Character _astop_down_character))
  (EventDispatchers|AssignOnAbilitySwitched _output_get (delegate Custom|OnAbilitySwitched_Event_0))
  (bind _values (Utilities|Map|Values (Variables|Default|GetAbilities)))
  (for _array_element _values
    (bind _returnvalue (Game|SpawnActorfromClass _array_element (Math|Transform|MakeTransform "0, 0, 0") "AlwaysSpawn" (Components|GetOwner) 0))
    (Utilities|Array|Add (Variables|Default|GetAllAbilities) _returnvalue)))

(fn OnAbilityUsing
  (bind _selectedability (Variables|Default|GetSelectedAbility)
    (:then
      (bind (_output_get _canbeused) (Default|ReduceAbilityCapacity _selectedability))
      (return _output_get _canbeused))
    (:else)))

(fn OnAbilityRestoring
  (params (NewParam :type E_Effects%20Enum :default "NewEnumerator5"))
  (for _array_element (Variables|Default|GetAllAbilities)
    (if (Utilities|Enum|Equal(Enum) (.type (Variables|/Game/Blueprints/AbilitySystem/Abilities/BP_Ability.BP_Ability_C|GetAbilityInfo _array_element)) NewParam)
      (LocalVariables|SetNewLocalVar_0 _array_element)))
  (bind (_output_get _returnvalue) (Default|RestoreAbility (LocalVariables|GetNewLocalVar_0)))
  (return _output_get _returnvalue))